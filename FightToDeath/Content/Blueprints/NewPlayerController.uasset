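; Player controller for a local two-player fighting game, routing keyboard/mouse to character 0 and gamepad to character 1.
; Input drives crouch, respawn and left/right punches, which set ThirdPersonCharacter flags and enable Sphere collision.
; BeginPlay adds health bar, death and victory widgets to the player screen with short delays.
; Tick, gated by a 20-second Delay, shows the victory widget on TwoPlayerMap when neither character is dead; its else branch repeats that same check.
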(event EventBeginPlay
  (Utilities|FlowControl|Delay 0.1)
  (bind _returnvalue (UserInterface|CreateWidget "/Game/ThirdPersonBP/Widgets/HelathBarHUD.HelathBarHUD_C" self))
  (bind _output_get (Variables|Default|SetHUDPC _returnvalue))
  (UserInterface|Viewport|AddtoPlayerScreen _output_get)
  (Utilities|FlowControl|Delay 0.1)
  (bind _returnvalue_2 (UserInterface|CreateWidget "/Game/ThirdPersonBP/Widgets/DeathWidget.DeathWidget_C" self))
  (UserInterface|Viewport|AddtoPlayerScreen _returnvalue_2)
  (Utilities|FlowControl|Delay 0.1)
  (bind _returnvalue_3 (UserInterface|CreateWidget "/Game/ThirdPersonBP/Widgets/VictoryWidget.VictoryWidget_C" self))
  (bind _output_get_2 (Variables|Default|SetVictoryWidget _returnvalue_3))
  (UserInterface|Viewport|AddtoPlayerScreen _output_get_2))

(event EventTick
  (params (DeltaSeconds :type Float%20%28single-precision%29))
  (Utilities|FlowControl|Delay 2e+01)
  (bind _returnvalue (Game|GetCurrentLevelName true))
  (if (Utilities|Enum|Equal(Enum) _returnvalue "TwoPlayerMap")
    (bind _asthird_person_character (Utilities|Casting|CastToThirdPersonCharacter (Game|GetPlayerCharacter 1)))
    (bind _asthird_person_character_2 (Utilities|Casting|CastToThirdPersonCharacter (Game|GetPlayerCharacter 0)))
    (bind _foundwidgets (Widget|GetAllWidgetsOfClass "/Game/ThirdPersonBP/Widgets/VictoryWidget.VictoryWidget_C" true))
    (if (and (Math|Boolean|Equal(Boolean) (Variables|/Game/ThirdPersonBP/Blueprints/ThirdPersonCharacter.ThirdPersonCharacter_C|GetIs%20Dead _asthird_person_character) false) (Math|Boolean|NotEqual(Boolean) (Variables|/Game/ThirdPersonBP/Blueprints/ThirdPersonCharacter.ThirdPersonCharacter_C|GetIs%20Dead _asthird_person_character_2) true))
      (Widget|SetVisibility (Utilities|Array|Get(acopy) _foundwidgets) "Visible")
      (elif (and (Math|Boolean|Equal(Boolean) (Variables|/Game/ThirdPersonBP/Blueprints/ThirdPersonCharacter.ThirdPersonCharacter_C|GetIs%20Dead _asthird_person_character) false) (Math|Boolean|NotEqual(Boolean) (Variables|/Game/ThirdPersonBP/Blueprints/ThirdPersonCharacter.ThirdPersonCharacter_C|GetIs%20Dead _asthird_person_character_2) true))
        (Widget|SetVisibility (Utilities|Array|Get(acopy) _foundwidgets) "Visible")))))

(event Input|GamepadEvents|GamepadFaceButtonTop
  (params (Key :type Key%20Structure))
  (:Released
    (Default|Respawn (.AsThird%20Person%20Character (Utilities|Casting|CastToThirdPersonCharacter (Game|GetPlayerCharacter 1))))))

(event Input|GamepadEvents|GamepadFaceButtonLeft
  (params (Key :type Key%20Structure))
  (bind _returnvalue (Game|GetPlayerCharacter 1))
  (:Pressed
    (Character|Crouch _returnvalue))
  (:Released
    (Character|UnCrouch _returnvalue)))

(event Input|GamepadEvents|GamepadLeftTrigger
  (params (Key :type Key%20Structure))
  (bind _returnvalue (Game|GetPlayerCharacter 1))
  (bind _asthird_person_character (Utilities|Casting|CastToThirdPersonCharacter _returnvalue))
  (:Pressed
    (Variables|/Game/ThirdPersonBP/Blueprints/ThirdPersonCharacter.ThirdPersonCharacter_C|SetisPunchingLeft _asthird_person_character true)
    (Collision|SetCollisionEnabled (Variables|/Game/ThirdPersonBP/Blueprints/ThirdPersonCharacter.ThirdPersonCharacter_C|GetSphere _asthird_person_character) "QueryAndPhysics")))

(event Input|GamepadEvents|GamepadRightTrigger
  (params (Key :type Key%20Structure))
  (bind _returnvalue (Game|GetPlayerCharacter 1))
  (bind _asthird_person_character (Utilities|Casting|CastToThirdPersonCharacter _returnvalue))
  (:Pressed
    (Variables|/Game/ThirdPersonBP/Blueprints/ThirdPersonCharacter.ThirdPersonCharacter_C|SetisPunchingRight _asthird_person_character true)
    (Collision|SetCollisionEnabled (Variables|/Game/ThirdPersonBP/Blueprints/ThirdPersonCharacter.ThirdPersonCharacter_C|GetSphere _asthird_person_character) "QueryAndPhysics")))

(event Input|KeyboardEvents|R
  (params (Key :type Key%20Structure))
  (:Released
    (Default|Respawn (.AsThird%20Person%20Character (Utilities|Casting|CastToThirdPersonCharacter (Game|GetPlayerCharacter 0))))))

(event Input|KeyboardEvents|LeftCtrl
  (params (Key :type Key%20Structure))
  (bind _returnvalue (Game|GetPlayerCharacter 0))
  (:Pressed
    (Character|Crouch _returnvalue))
  (:Released
    (Character|UnCrouch _returnvalue)))

(event Input|MouseEvents|LeftMouseButton
  (params (Key :type Key%20Structure))
  (bind _returnvalue (Game|GetPlayerCharacter 0))
  (bind _asthird_person_character (Utilities|Casting|CastToThirdPersonCharacter _returnvalue))
  (:Pressed
    (Variables|/Game/ThirdPersonBP/Blueprints/ThirdPersonCharacter.ThirdPersonCharacter_C|SetisPunchingLeft _asthird_person_character true)
    (Collision|SetCollisionEnabled (Variables|/Game/ThirdPersonBP/Blueprints/ThirdPersonCharacter.ThirdPersonCharacter_C|GetSphere _asthird_person_character) "QueryAndPhysics")))

(event Input|MouseEvents|RightMouseButton
  (params (Key :type Key%20Structure))
  (bind _returnvalue (Game|GetPlayerCharacter 0))
  (bind _asthird_person_character (Utilities|Casting|CastToThirdPersonCharacter _returnvalue))
  (:Pressed
    (Variables|/Game/ThirdPersonBP/Blueprints/ThirdPersonCharacter.ThirdPersonCharacter_C|SetisPunchingRight _asthird_person_character true)
    (Collision|SetCollisionEnabled (Variables|/Game/ThirdPersonBP/Blueprints/ThirdPersonCharacter.ThirdPersonCharacter_C|GetSphere _asthird_person_character) "QueryAndPhysics")))

(fn ConstructionScript)